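; Interactable fisherman character who gets pushed and ends up floating dead in the water.
; Interact plays a Wilhelm scream and the pushed montage, then a timeline lerps the skeletal mesh to the EndRefLoc marker with a growing downward offset.
; A second timeline raises the mesh back up, then a looping dead-in-water animation takes over.
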(event `/Game/Blueprints/InteractionCharacters/I_Interactable.Interact`
  (bind _actorstartloc (`self.ActorStartLoc`))
  (bind _skeletalmesh (`self.SkeletalMesh`))
  (bind _returnvalue (`SceneComponent.K2_GetComponentLocation` (`self.SkeletalMesh`)))
  (`parent.Interact`)
  (set `self.ActorStartLoc` _returnvalue)
  (`GameplayStatics.PlaySoundAtLocation` "/Game/Sounds/Man/VOXScrm_Wilhelm_scream__ID_0477__BSB_Cue.VOXScrm_Wilhelm_scream__ID_0477__BSB_Cue" _returnvalue (struct) 1.0 1.0 0.0 null null null null)
  (`SkeletalMeshComponent.SetAnimation` _skeletalmesh "/Game/Characters/Fisherman/Animations/AM_Pushed.AM_Pushed")
  (`|PlayMontage` _skeletalmesh "/Game/Characters/Fisherman/Animations/AM_Pushed.AM_Pushed"
    (:`then`
      (bind (_direction _newtrack_0) (`Timeline|Timeline`)
        (:`Update`
          (`SceneComponent.K2_SetWorldLocation` (`self.SkeletalMesh`) (`KismetMathLibrary.VLerp` (`self.ActorStartLoc`) (- (`SceneComponent.K2_GetComponentLocation` (`self.EndRefLoc`)) (`KismetMathLibrary.MakeVector` 0.0 0.0 (`KismetMathLibrary.Lerp` 10.0 50.0 _newtrack_0))) _newtrack_0) false false))
        (:`Finished`
          (set `self.ActorStartLoc` (`SceneComponent.K2_GetComponentLocation` (`self.SkeletalMesh`)))
          (bind (_direction_2 _newtrack_0_2) (`Timeline|Timeline_0`)
            (:`Update`
              (`SceneComponent.K2_SetWorldLocation` (`self.SkeletalMesh`) (`KismetMathLibrary.VLerp` _actorstartloc (+ _actorstartloc (0.0 0.0 100.0)) _newtrack_0_2) false false))
            (:`Finished`
              (`SkeletalMeshComponent.PlayAnimation` (`self.SkeletalMesh`) "/Game/Characters/Fisherman/Animations/Fisherman_CharacterArmature_DeadInWater.Fisherman_CharacterArmature_DeadInWater" true))))))))

(fn `UserConstructionScript`
  (`parent.UserConstructionScript`))