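; Interactable lumberjack whose Interact event makes a tree fall and the character die.
; Interacting runs the parent logic and plays a Wilhelm scream at the skeletal mesh.
; A timeline lerps the tree from its current relative transform toward a TreeEndRef marker, while the death montage plays sped up after a short delay.
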(event `/Game/Blueprints/InteractionCharacters/I_Interactable.Interact`
  (bind _tree (`self.Tree`))
  (bind _skeletalmesh (`self.SkeletalMesh`))
  (bind (_returnvalue_location _returnvalue_rotation) (`KismetMathLibrary.BreakTransform` (`SceneComponent.GetRelativeTransform` (`self.TreeEndRef`))))
  (bind (_returnvalue_location_2 _returnvalue_rotation_2) (`KismetMathLibrary.BreakTransform` (`SceneComponent.GetRelativeTransform` _tree)))
  (`parent.Interact`)
  (`GameplayStatics.PlaySoundAtLocation` "/Game/Sounds/Man/VOXScrm_Wilhelm_scream__ID_0477__BSB_Cue.VOXScrm_Wilhelm_scream__ID_0477__BSB_Cue" (`SceneComponent.K2_GetComponentLocation` (`self.SkeletalMesh`)) (struct) 1.0 1.0 0.0 null null null null)
  (`|ExecutionSequence`
    (:`then_0`
      (`KismetSystemLibrary.Delay` 0.2)
      (`SkeletalMeshComponent.SetAnimation` _skeletalmesh "/Game/Characters/LumberJack/Animations/AM_Dead.AM_Dead")
      (`|PlayMontage` _skeletalmesh "/Game/Characters/LumberJack/Animations/AM_Dead.AM_Dead" 2.0))
    (:`then_1`
      (bind (_direction _newtrack_0) (`Timeline|TreeFall`)
        (:`Update`
          (`SceneComponent.K2_SetRelativeLocationAndRotation` _tree (`KismetMathLibrary.VLerp` _returnvalue_location_2 _returnvalue_location _newtrack_0) (`KismetMathLibrary.RLerp` _returnvalue_rotation_2 _returnvalue_rotation _newtrack_0) false false))))))

(fn `UserConstructionScript`
  (`parent.UserConstructionScript`))