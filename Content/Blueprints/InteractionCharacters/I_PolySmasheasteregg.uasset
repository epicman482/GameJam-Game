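; I_PolySmasheasteregg is an interactable easter egg where interacting plays a punch and scream and topples a tree.
; Interact disables its collision and hides both interaction widgets, then plays the TreeFall timeline.
; Each update lerps the tree from its current relative location and rotation toward the TreeEndRef marker.
; A DoOnce on that update path plays the tree-fall sound only once.
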(event `/Game/Blueprints/InteractionCharacters/I_Interactable.Interact`
  (bind _tree (`self.Tree`))
  (bind (_returnvalue_location _returnvalue_rotation) (`KismetMathLibrary.BreakTransform` (`SceneComponent.GetRelativeTransform` (`self.TreeEndRef`))))
  (bind (_returnvalue_location_2 _returnvalue_rotation_2) (`KismetMathLibrary.BreakTransform` (`SceneComponent.GetRelativeTransform` _tree)))
  (`GameplayStatics.PlaySoundAtLocation` "/Game/Sounds/Man/Punch/Punch_Cue.Punch_Cue" (`self.K2_GetActorLocation` (`self.BP Third Person CharacterRef`)) (struct) 1.0 1.0 0.0 null null null null)
  (`PrimitiveComponent.SetCollisionEnabled` (`self.CollisionBox`) "NoCollision")
  (`PrimitiveComponent.SetCollisionEnabled` (`self.Sphere`) "NoCollision")
  (`SceneComponent.SetVisibility` (`self.InteractWidget`) false false)
  (`SceneComponent.SetVisibility` (`self.InteractNotifWidget`) false false)
  (`GameplayStatics.PlaySoundAtLocation` "/Game/Sounds/Man/Scream/Scream_Cue.Scream_Cue" (`SceneComponent.K2_GetComponentLocation` (`self.SkeletalMesh`)) (struct) 1.0 1.0 0.0 null null null null)
  (bind (_direction _newtrack_0) (`Timeline|TreeFall`)
    (:`Update`
      (`|ExecutionSequence`
        (:`then_0`
          (`SceneComponent.K2_SetRelativeLocationAndRotation` _tree (`KismetMathLibrary.VLerp` _returnvalue_location_2 _returnvalue_location _newtrack_0) (`KismetMathLibrary.RLerp` _returnvalue_rotation_2 _returnvalue_rotation _newtrack_0) false false))
        (:`then_1`
          (`/Engine/EditorBlueprintResources/StandardMacros.DoOnce` false
            (:`Completed`
              (`GameplayStatics.PlaySoundAtLocation` "/Game/Sounds/Enviroment/Tree/Treefall_Cue.Treefall_Cue" (`SceneComponent.K2_GetComponentLocation` (`self.Tree`)) (struct) 1.0 1.0 0.0 null null null null))))))))

(fn `UserConstructionScript`
  (`parent.UserConstructionScript`))