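; Parent Blueprint for interactible actors that the player can punch, each interaction counting toward a kill tally.
; An outer Sphere overlap shows a notification widget; the CollisionBox overlap swaps it for the interact prompt and sets IsInteractingActive on the cached player character.
; Interact plays a punch sound, disables both collision volumes, hides both widgets, increments PeopleKills and refreshes the kill counter if its own KillWidget is invalid.
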(event `self.ReceiveBeginPlay`
  (bind _asbp_third_person_character (cast `/Game/ThirdPerson/Blueprints/BP_ThirdPersonCharacter` (`GameplayStatics.GetPlayerPawn` 0)))
  (set `self.BP Third Person CharacterRef` _asbp_third_person_character))

(event `self.CollisionBox.OnComponentBeginOverlap`
  (params (OverlappedComponent :type "PrimitiveComponent Object Reference") (OtherActor :type "Actor Object Reference") (OtherComp :type "PrimitiveComponent Object Reference") (OtherBodyIndex :type Integer) (bFromSweep :type Boolean) (SweepResult :type "HitResult Structure (by ref)"))
  (bind _output_get (set `self.Other Actor` OtherActor))
  (if (== _output_get (`GameplayStatics.GetPlayerPawn` 0))
    (set `/Game/ThirdPerson/Blueprints/BP_ThirdPersonCharacter.IsInteractingActive?` true (`self.BP Third Person CharacterRef`))
    (`SceneComponent.SetVisibility` (`self.InteractWidget`) true false)
    (`SceneComponent.SetVisibility` (`self.InteractNotifWidget`) false false)
    (`KismetSystemLibrary.PrintString` "Collided")))

(event `self.CollisionBox.OnComponentEndOverlap`
  (params (OverlappedComponent :type "PrimitiveComponent Object Reference") (OtherActor :type "Actor Object Reference") (OtherComp :type "PrimitiveComponent Object Reference") (OtherBodyIndex :type Integer))
  (bind _output_get (set `self.Other Actor` OtherActor))
  (if (== _output_get (`GameplayStatics.GetPlayerPawn` 0))
    (set `/Game/ThirdPerson/Blueprints/BP_ThirdPersonCharacter.IsInteractingActive?` false (`self.BP Third Person CharacterRef`))
    (`SceneComponent.SetVisibility` (`self.InteractWidget`) false false)
    (`SceneComponent.SetVisibility` (`self.InteractNotifWidget`) true false)
    (`KismetSystemLibrary.PrintString` "StopCollided")))

(event `self.Sphere.OnComponentBeginOverlap`
  (params (OverlappedComponent :type "PrimitiveComponent Object Reference") (OtherActor :type "Actor Object Reference") (OtherComp :type "PrimitiveComponent Object Reference") (OtherBodyIndex :type Integer) (bFromSweep :type Boolean) (SweepResult :type "HitResult Structure (by ref)"))
  (bind _output_get (set `self.Other Actor` OtherActor))
  (if (== _output_get (`GameplayStatics.GetPlayerPawn` 0))
    (`SceneComponent.SetVisibility` (`self.InteractNotifWidget`) true false)))

(event `self.Sphere.OnComponentEndOverlap`
  (params (OverlappedComponent :type "PrimitiveComponent Object Reference") (OtherActor :type "Actor Object Reference") (OtherComp :type "PrimitiveComponent Object Reference") (OtherBodyIndex :type Integer))
  (bind _output_get (set `self.Other Actor` OtherActor))
  (if (== _output_get (`GameplayStatics.GetPlayerPawn` 0))
    (`SceneComponent.SetVisibility` (`self.InteractNotifWidget`) false false)))

(event `/Game/Blueprints/InteractionCharacters/I_Interactable.Interact`
  (bind _bp_third_person_characterref (`self.BP Third Person CharacterRef`))
  (`GameplayStatics.PlaySoundAtLocation` "/Game/Sounds/Man/Punch/Punch_Cue.Punch_Cue" (`self.K2_GetActorLocation` (`self.BP Third Person CharacterRef`)) (struct) 1.0 1.0 0.0 null null null null)
  (`PrimitiveComponent.SetCollisionEnabled` (`self.CollisionBox`) "NoCollision")
  (`PrimitiveComponent.SetCollisionEnabled` (`self.Sphere`) "NoCollision")
  (`SceneComponent.SetVisibility` (`self.InteractWidget`) false false)
  (`SceneComponent.SetVisibility` (`self.InteractNotifWidget`) false false)
  (set `/Game/ThirdPerson/Blueprints/BP_ThirdPersonCharacter.PeopleKills` (+ (`/Game/ThirdPerson/Blueprints/BP_ThirdPersonCharacter.PeopleKills` _bp_third_person_characterref) 1) _bp_third_person_characterref)
  (`/Engine/EditorBlueprintResources/StandardMacros.IsValid` (`self.KillWidget`)
    (:`Is Not Valid`
      (`/Game/Widgets/WIdgetkills/KillWidget.UpdateKillCounter` (`/Game/ThirdPerson/Blueprints/BP_ThirdPersonCharacter.KillWidgetRef` _bp_third_person_characterref)))))

(fn `UserConstructionScript`)