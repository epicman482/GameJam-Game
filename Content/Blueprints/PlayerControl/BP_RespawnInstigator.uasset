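; BP_RespawnInstigator is a trigger actor that sends the player back to their respawn location on overlap.
; It caches the player's BP_ThirdPersonCharacter on BeginPlay.
; When the player pawn enters its Box, it moves the character to that character's stored RespawnLoc and zeroes its movement velocity so no momentum carries over.
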(event `self.ReceiveBeginPlay`
  (bind _asbp_third_person_character (cast `/Game/ThirdPerson/Blueprints/BP_ThirdPersonCharacter` (`GameplayStatics.GetPlayerPawn` 0)))
  (set `self.BP Third Person CharacterRef` _asbp_third_person_character))

(event `self.Box.OnComponentBeginOverlap`
  (params (OverlappedComponent :type "PrimitiveComponent Object Reference") (OtherActor :type "Actor Object Reference") (OtherComp :type "PrimitiveComponent Object Reference") (OtherBodyIndex :type Integer) (bFromSweep :type Boolean) (SweepResult :type "HitResult Structure (by ref)"))
  (bind _bp_third_person_characterref (`self.BP Third Person CharacterRef`))
  (bind _output_get (set `self.Other Actor` OtherActor))
  (if (== _output_get (`GameplayStatics.GetPlayerPawn` 0))
    (`self.K2_SetActorLocation` _bp_third_person_characterref (`/Game/ThirdPerson/Blueprints/BP_ThirdPersonCharacter.RespawnLoc` _bp_third_person_characterref) false false)
    (set `MovementComponent.Velocity` (0.0 0.0 0.0) (`Character.CharacterMovement` _bp_third_person_characterref))))

(fn `UserConstructionScript`)